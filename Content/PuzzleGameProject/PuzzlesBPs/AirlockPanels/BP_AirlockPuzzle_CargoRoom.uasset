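; BP_AirlockPuzzle_CargoRoom is a three-ring rotation puzzle that unlocks the cargo room door by turning off its collision.
; AirlockInteraction rolls the given ring left or right by a fixed step and prints its rotation.
; CheckCombination compares that ring's roll to its target with a small tolerance and stores the per-ring result.
; When every stored result is correct, it finds BP_DoorCargoRoom by class and calls CollisionOff.
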(event `/Game/PuzzleGameProject/PuzzlesBPs/AirlockPanels/AirlocksInterface.AirlockInteraction`
  (params (Rings :type "PrimitiveComponent Object Reference") (RotateLeft :type Boolean))
  (`self.Rotate` Rings RotateLeft))

(fn `CheckCombination`
  (params (Rings :type "PrimitiveComponent Object Reference"))
  (locals (SelectedRing :type Integer) (IncorrectCombination :type Boolean) (NewLocalVar :type "PrimitiveComponent Object Reference"))
  (bind _relativerotation_roll (`KismetMathLibrary.BreakRotator` (`SceneComponent.RelativeRotation` Rings)))
  (if (== Rings (`self.InnerRing`))
    (set `local.SelectedRing` 0)
    (`KismetArrayLibrary.Array_Set` (`self.CorrectCombination`) (`local.SelectedRing`) (`KismetMathLibrary.NearlyEqual_FloatFloat` (`|GetArrayItem` (`self.Combination`) (`local.SelectedRing`)) _relativerotation_roll 1.0) :!label _label)
    (for _array_element (`self.CorrectCombination`)
      (if (not _array_element)
        (set `local.IncorrectCombination` true)
        (break)))
    (if (not (`local.IncorrectCombination`))
      (bind _returnvalue (`GameplayStatics.GetActorOfClass` "/Game/Repair_Tool/DoorCollision/BP_DoorCargoRoom.BP_DoorCargoRoom_C"))
      (`/Game/Repair_Tool/DoorCollision/BP_DoorCargoRoom.CollisionOff` _returnvalue))
    (elif (== Rings (`self.MiddleRing`))
      (set `local.SelectedRing` 1)
      (goto _label)
      (elif (== Rings (`self.OuterRing`))
        (set `local.SelectedRing` 2)
        (goto _label)))))

(fn `Rotate`
  (params (Rings :type "PrimitiveComponent Object Reference") (RotateLeft :type Boolean))
  (bind _rotationvalue (`self.RotationValue`))
  (if RotateLeft
    (`SceneComponent.K2_AddRelativeRotation` Rings (`KismetMathLibrary.MakeRotator` (* _rotationvalue -1.0)) false false)
    (else
      (`SceneComponent.K2_AddRelativeRotation` Rings (`KismetMathLibrary.MakeRotator` _rotationvalue) false false)))
  (`KismetSystemLibrary.PrintString` (`KismetStringLibrary.Conv_RotatorToString` (`SceneComponent.RelativeRotation` Rings)))
  (`self.CheckCombination` Rings))

(fn `UserConstructionScript`)