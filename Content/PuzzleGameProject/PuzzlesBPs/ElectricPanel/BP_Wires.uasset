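; Electric panel wire-matching puzzle that powers tubes and triggers generator door logic when solved.
; Construction gathers four coloured BP_Wire child actors; BeginPlay shuffles their attach targets and binds each attach event to a completion check.
; Success electrifies tube materials, blends back to the first-person camera, restores gun and HUD, notifies both door actors and removes the interaction trigger.
; Box overlaps toggle the player's AbleToActivate flag, and a looping timer spins a counter while Activated.
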(event `self.ReceiveBeginPlay`
  (`self.ShuffleEndLocation`)
  (for _array_element (`self.Wires`)
    (add `/Game/PuzzleGameProject/PuzzlesBPs/ElectricPanel/BP_Wire.OnAttached` _array_element (delegate `OnAttached_Event`))))

(event `OnAttached_Event`
  (bind _returnvalue (`GameplayStatics.GetPlayerController` 0))
  (if (`self.IsCompleted`)
    (bind _returnvalue_2 (`GameplayStatics.GetActorOfClass` "/Game/PuzzleGameProject/Shader/Blueprints/BP_TubesShader1.BP_TubesShader1_C"))
    (`PrimitiveComponent.SetMaterial` (`/Game/PuzzleGameProject/Shader/Blueprints/BP_TubesShader1.Tube2_Annabelle` _returnvalue_2) 0 "/Game/PuzzleGameProject/Shader/MI_Electricity.MI_Electricity")
    (bind _returnvalue_3 (`GameplayStatics.GetActorOfClass` "/Game/PuzzleGameProject/Shader/Blueprints/BP_TubesShader2.BP_TubesShader2_C"))
    (`PrimitiveComponent.SetMaterial` (`/Game/PuzzleGameProject/Shader/Blueprints/BP_TubesShader2.Tube2_Annabelle` _returnvalue_3) 0 "/Game/PuzzleGameProject/Shader/MI_Electricity.MI_Electricity")
    (`GameplayStatics.PlaySound2D` "/Game/Repair_Tool/Music/WiresConnected.WiresConnected" 1.0 1.0 0.0 null null)
    (`KismetSystemLibrary.PrintString` "Completed!" true true (struct :`R` 1.0 :`G` 1.0 :`B` 1.0 :`A` 1.0))
    (bind _asbp_first_person_character (cast `/Game/FirstPerson/Blueprints/BP_FirstPersonCharacter` (`GameplayStatics.GetPlayerPawn` 0)))
    (`PlayerController.SetViewTargetWithBlend` _returnvalue (`ActorComponent.GetOwner` (`/Game/FirstPerson/Blueprints/BP_FirstPersonCharacter.FirstPersonCamera` _asbp_first_person_character)) 0.4 "VTBlend_Linear" 0.0 false)
    (set `PlayerController.bShowMouseCursor` false _returnvalue)
    (set `/Game/FirstPerson/Blueprints/BP_FirstPersonCharacter.PanelView?` false _asbp_first_person_character)
    (`/Game/FirstPerson/Blueprints/BP_FirstPersonCharacter.GunVisibilityOn` _asbp_first_person_character)
    (bind _returnvalue_4 (`GameplayStatics.GetActorOfClass` "/Game/PuzzleGameProject/PuzzlesBPs/ElectricPanel/WiresWidget1.WiresWidget1_C"))
    (`self.K2_DestroyActor` _returnvalue_4)
    (bind _foundwidgets (`WidgetBlueprintLibrary.GetAllWidgetsOfClass` "/Game/Repair_Tool/HUD_Paralax/WB_HUD.WB_HUD_C"))
    (`Widget.SetVisibility` _foundwidgets "Visible")
    (bind _returnvalue_5 (`GameplayStatics.GetActorOfClass` "/Game/Repair_Tool/DoorCollision/BP_DoorGenerator1.BP_DoorGenerator1_C"))
    (`/Game/Repair_Tool/DoorCollision/BP_DoorGenerator1.CollisionLocationDoorON` _returnvalue_5)
    (bind _returnvalue_6 (`GameplayStatics.GetActorOfClass` "/Game/Repair_Tool/DoorCollision/BP_DoorSmallGenerator1.BP_DoorSmallGenerator1_C"))
    (`/Game/Repair_Tool/DoorCollision/BP_DoorSmallGenerator1.LocationOn` _returnvalue_6)
    (`ActorComponent.K2_DestroyComponent` (`self.Box1`))))

(event `StartTimer`
  (bind _returnvalue (`KismetSystemLibrary.K2_SetTimerDelegate` (delegate `UpdateTimer`) 0.1 true))
  (set `self.RotationTimer` _returnvalue))

(event `UpdateTimer`
  (if (`self.Activated?`)
    (`SceneComponent.K2_AddLocalRotation` (`self.Counter1`) (struct :`Roll` 15.0) false false)))

(event `StopTimer`
  (`SceneComponent.K2_SetRelativeRotation` :`self` (`self.Counter1`))
  (set `self.Activated?` false)
  (`KismetSystemLibrary.K2_PauseTimerHandle` (`self.RotationTimer`)))

(event `self.Box1.OnComponentBeginOverlap`
  (params (OverlappedComponent :type "PrimitiveComponent Object Reference") (OtherActor :type "Actor Object Reference") (OtherComp :type "PrimitiveComponent Object Reference") (OtherBodyIndex :type Integer) (bFromSweep :type Boolean) (SweepResult :type "HitResult Structure (by ref)"))
  ;[1 1 1] Swapping Cameras
  (bind _asbp_first_person_character (cast `/Game/FirstPerson/Blueprints/BP_FirstPersonCharacter` OtherActor))
  (set `/Game/FirstPerson/Blueprints/BP_FirstPersonCharacter.AbleToActivate` true _asbp_first_person_character))

(event `self.Box1.OnComponentEndOverlap`
  (params (OverlappedComponent :type "PrimitiveComponent Object Reference") (OtherActor :type "Actor Object Reference") (OtherComp :type "PrimitiveComponent Object Reference") (OtherBodyIndex :type Integer))
  ;[1 1 1] Swapping Cameras
  (bind _asbp_first_person_character (cast `/Game/FirstPerson/Blueprints/BP_FirstPersonCharacter` OtherActor))
  (set `/Game/FirstPerson/Blueprints/BP_FirstPersonCharacter.AbleToActivate` false _asbp_first_person_character))

(fn `IsCompleted`
  (returns (Completed :type Boolean))
  (locals (IsSuccessArray :type "Array of Boolean"))
  (for _array_element (`self.Wires`)
    (`KismetArrayLibrary.Array_Add` (`local.IsSuccessArray`) (`/Game/PuzzleGameProject/PuzzlesBPs/ElectricPanel/BP_Wire.IsSuccess` _array_element)))
  (return (not (`KismetArrayLibrary.Array_Contains` (`local.IsSuccessArray`)))))

(fn `ShuffleEndLocation`
  (locals (Locations :type "Array of Vector Structure"))
  (`|ExecutionSequence`
    (:`then_0`
      (for _array_element (`self.Wires`)
        (`KismetArrayLibrary.Array_Add` (`local.Locations`) (`/Game/PuzzleGameProject/PuzzlesBPs/ElectricPanel/BP_Wire.GetAttachLocation` _array_element))))
    (:`then_1`
      (`KismetArrayLibrary.Array_Shuffle` (`local.Locations`)))
    (:`then_2`
      (for (_array_element_2 _array_index) (`self.Wires`)
        (`/Game/PuzzleGameProject/PuzzlesBPs/ElectricPanel/BP_Wire.SetAttachLocation` _array_element_2 (`|GetArrayItem` (`local.Locations`) _array_index))))))

(fn `UserConstructionScript`
  (`|ExecutionSequence`
    (:`then_0`
      (for _array_element (`|MakeArray` (`self.RedWire`) (`self.BlueWire`) (`self.GreenWire`) (`self.YellowWire`))
        (bind _asbp_wire (cast `/Game/PuzzleGameProject/PuzzlesBPs/ElectricPanel/BP_Wire` (`ChildActorComponent.ChildActor` _array_element)))
        (`KismetArrayLibrary.Array_Add` (`self.Wires`) _asbp_wire)))
    (:`then_1`
      (for (_array_element_2 _array_index) (`self.Wires`)
        (`/Game/PuzzleGameProject/PuzzlesBPs/ElectricPanel/BP_Wire.SetWireColour` _array_element_2 (`|GetArrayItem` (`self.Colours`) _array_index))))))