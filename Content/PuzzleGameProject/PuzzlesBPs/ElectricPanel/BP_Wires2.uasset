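; Electric panel wire puzzle actor that, when all wires attach successfully, prints completion, disables collision on the BP_BarrierElectricRoom1 box and destroys its own trigger.
; Construction gathers four colored BP_Wire child actors; BeginPlay shuffles their attach locations and binds their OnAttached events to the completion check.
; Box2 overlaps toggle the first-person character's AbleToActivate2 flag.
; Timer events spin Counter2 while Activated2 is set, then reset and pause it.
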(event `self.ReceiveBeginPlay`
  (`self.ShuffleEndLocation`)
  (for _array_element (`self.Wires`)
    (add `/Game/PuzzleGameProject/PuzzlesBPs/ElectricPanel/BP_Wire.OnAttached` _array_element (delegate `OnAttached_Event`))))

(event `StartTimer2`
  (bind _returnvalue (`KismetSystemLibrary.K2_SetTimerDelegate` (delegate `UpdateTimer2`) 0.1 true))
  (set `self.RotationTimer2` _returnvalue))

(event `OnAttached_Event`
  (if (`self.IsCompleted`)
    (`KismetSystemLibrary.PrintString` "Completed!" true true (struct :`R` 1.0 :`G` 1.0 :`B` 1.0 :`A` 1.0))
    (bind _returnvalue (`GameplayStatics.GetActorOfClass` "/Game/Repair_Tool/DoorCollision/BP_BarrierElectricRoom1.BP_BarrierElectricRoom1_C"))
    (`PrimitiveComponent.SetCollisionEnabled` (`/Game/Repair_Tool/DoorCollision/BP_BarrierElectricRoom1.Box` _returnvalue) "NoCollision")
    (`ActorComponent.K2_DestroyComponent` (`self.Box2`))))

(event `UpdateTimer2`
  (if (`self.Activated2?`)
    (`SceneComponent.K2_AddLocalRotation` (`self.Counter2`) (struct :`Roll` 15.0) false false)))

(event `StopTimer2`
  (`SceneComponent.K2_SetRelativeRotation` :`self` (`self.Counter2`))
  (set `self.Activated2?` false)
  (`KismetSystemLibrary.K2_PauseTimerHandle` (`self.RotationTimer2`)))

(event `self.Box2.OnComponentBeginOverlap`
  (params (OverlappedComponent :type "PrimitiveComponent Object Reference") (OtherActor :type "Actor Object Reference") (OtherComp :type "PrimitiveComponent Object Reference") (OtherBodyIndex :type Integer) (bFromSweep :type Boolean) (SweepResult :type "HitResult Structure (by ref)"))
  ;[1 1 1] Swapping Cameras
  (bind _asbp_first_person_character (cast `/Game/FirstPerson/Blueprints/BP_FirstPersonCharacter` OtherActor))
  (bind _output_get (set `/Game/FirstPerson/Blueprints/BP_FirstPersonCharacter.AbleToActivate2` true _asbp_first_person_character))
  (`KismetSystemLibrary.PrintString` (`KismetStringLibrary.Conv_BoolToString` _output_get)))

(event `self.Box2.OnComponentEndOverlap`
  (params (OverlappedComponent :type "PrimitiveComponent Object Reference") (OtherActor :type "Actor Object Reference") (OtherComp :type "PrimitiveComponent Object Reference") (OtherBodyIndex :type Integer))
  ;[1 1 1] Swapping Cameras
  (bind _asbp_first_person_character (cast `/Game/FirstPerson/Blueprints/BP_FirstPersonCharacter` OtherActor))
  (bind _output_get (set `/Game/FirstPerson/Blueprints/BP_FirstPersonCharacter.AbleToActivate2` false _asbp_first_person_character))
  (`KismetSystemLibrary.PrintString` (`KismetStringLibrary.Conv_BoolToString` _output_get)))

(fn `IsCompleted`
  (returns (Completed :type Boolean))
  (locals (IsSuccessArray :type "Array of Boolean"))
  (for _array_element (`self.Wires`)
    (`KismetArrayLibrary.Array_Add` (`local.IsSuccessArray`) (`/Game/PuzzleGameProject/PuzzlesBPs/ElectricPanel/BP_Wire.IsSuccess` _array_element)))
  (return (not (`KismetArrayLibrary.Array_Contains` (`local.IsSuccessArray`)))))

(fn `ShuffleEndLocation`
  (locals (Locations :type "Array of Vector Structure"))
  (`|ExecutionSequence`
    (:`then_0`
      (for _array_element (`self.Wires`)
        (`KismetArrayLibrary.Array_Add` (`local.Locations`) (`/Game/PuzzleGameProject/PuzzlesBPs/ElectricPanel/BP_Wire.GetAttachLocation` _array_element))))
    (:`then_1`
      (`KismetArrayLibrary.Array_Shuffle` (`local.Locations`)))
    (:`then_2`
      (for (_array_element_2 _array_index) (`self.Wires`)
        (`/Game/PuzzleGameProject/PuzzlesBPs/ElectricPanel/BP_Wire.SetAttachLocation` _array_element_2 (`|GetArrayItem` (`local.Locations`) _array_index))))))

(fn `UserConstructionScript`
  (`|ExecutionSequence`
    (:`then_0`
      (for _array_element (`|MakeArray` (`self.RedWire`) (`self.BlueWire`) (`self.GreenWire`) (`self.YellowWire`))
        (bind _asbp_wire (cast `/Game/PuzzleGameProject/PuzzlesBPs/ElectricPanel/BP_Wire` (`ChildActorComponent.ChildActor` _array_element)))
        (`KismetArrayLibrary.Array_Add` (`self.Wires`) _asbp_wire)))
    (:`then_1`
      (for (_array_element_2 _array_index) (`self.Wires`)
        (`/Game/PuzzleGameProject/PuzzlesBPs/ElectricPanel/BP_Wire.SetWireColour` _array_element_2 (`|GetArrayItem` (`self.Colours`) _array_index))))))