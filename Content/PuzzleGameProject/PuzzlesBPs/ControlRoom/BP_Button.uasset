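; Control room puzzle button actor with a green (Button1) and a blue (Button3) button that pop back up after a push.
; PushGreen or PushBlue snaps its button to the body's location, resets ButtonPos and enables Tick.
; Tick raises both buttons regardless of which was pushed, advancing the shared counter for each, until it passes a limit and disables Tick.
; A Lerp-based ButtonAnimation and its transform setup are unused leftovers.
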(event `self.ReceiveBeginPlay`)

(event `self.ReceiveTick`
  (params (DeltaSeconds :type "Float (single-precision)"))
  (bind _button1 (`self.Button1`))
  (bind _buttonpos (`self.ButtonPos`))
  (bind _button3 (`self.Button3`))
  (bind _buttonpos_2 (`self.ButtonPos`))
  (bind (_relativelocation_x _relativelocation_y _relativelocation_z) (`KismetMathLibrary.BreakVector` (`SceneComponent.RelativeLocation` _button1)))
  (bind (_relativelocation_x_2 _relativelocation_y_2 _relativelocation_z_2) (`KismetMathLibrary.BreakVector` (`SceneComponent.RelativeLocation` _button3)))
  (`|ExecutionSequence`
    (:`then_0`
      (if true
        (`SceneComponent.K2_SetRelativeLocation` _button1 (`KismetMathLibrary.MakeVector` _relativelocation_x _relativelocation_y (+ _relativelocation_z 1.0)) false false)
        (if (> _buttonpos 5)
          (`self.SetActorTickEnabled` false)
          (else
            (`/Engine/EditorBlueprintResources/StandardMacros.IncrementInt` _buttonpos)))))
    (:`then_1`
      (if true
        (`SceneComponent.K2_SetRelativeLocation` _button3 (`KismetMathLibrary.MakeVector` _relativelocation_x_2 _relativelocation_y_2 (+ _relativelocation_z_2 1.0)) false false)
        (if (> _buttonpos_2 5)
          (`self.SetActorTickEnabled` false)
          (else
            (`/Engine/EditorBlueprintResources/StandardMacros.IncrementInt` _buttonpos_2)))))))

(event `/Game/PuzzleGameProject/PuzzlesBPs/ControlRoom/ButtonsInterface.PushGreen`
  (`SceneComponent.K2_SetRelativeLocation` (`self.Button1`) (`SceneComponent.RelativeLocation` (`self.ButtonBody1`)) false false)
  (`self.SetActorTickEnabled` true)
  (set `self.ButtonPos` 0))

(event `/Game/PuzzleGameProject/PuzzlesBPs/ControlRoom/ButtonsInterface.PushBlue`
  (`SceneComponent.K2_SetRelativeLocation` (`self.Button3`) (`SceneComponent.RelativeLocation` (`self.ButtonBody3`)) false false)
  (`self.SetActorTickEnabled` true)
  (set `self.ButtonPos` 0))

(fn `UserConstructionScript`)