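; BP_ButtonYellow is a yellow push button for the control room puzzle, animating its own press and release.
; PushButton snaps the Button component to the ButtonBody's relative location, resets a step counter and enables actor tick.
; Tick then raises the button one unit along Z per frame and disables itself once the counter passes its limit, so the return speed depends on frame rate.
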(event `self.ReceiveTick`
  (params (DeltaSeconds :type "Float (single-precision)"))
  (bind _button (`self.Button`))
  (bind _buttonpos (`self.ButtonPos`))
  (bind (_relativelocation_x _relativelocation_y _relativelocation_z) (`KismetMathLibrary.BreakVector` (`SceneComponent.RelativeLocation` _button)))
  (if true
    (`SceneComponent.K2_SetRelativeLocation` _button (`KismetMathLibrary.MakeVector` _relativelocation_x _relativelocation_y (+ _relativelocation_z 1.0)) false false)
    (if (> _buttonpos 5)
      (`self.SetActorTickEnabled` false)
      (else
        (`/Engine/EditorBlueprintResources/StandardMacros.IncrementInt` _buttonpos)))))

(event `/Game/PuzzleGameProject/PuzzlesBPs/ControlRoom/CR_Buttons_Interface.PushButton`
  (`SceneComponent.K2_SetRelativeLocation` (`self.Button`) (`SceneComponent.RelativeLocation` (`self.ButtonBody`)) false false)
  (`self.SetActorTickEnabled` true)
  (set `self.ButtonPos` 0))

(fn `UserConstructionScript`)