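; BP_Buttons is a control room puzzle button that has a press-in and pop-out animation.
; BeginPlay caches the mesh's resting transform and a lowered copy, then enables player input.
; Left mouse clicks feed a Gate leading to ButtonAnimation, where two chained timelines lerp between those transforms.
; The collision overlap events are empty, so nothing in the graph opens or closes the Gate.
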(event `self.ReceiveBeginPlay`
  (bind (_returnvalue_location _returnvalue_rotation _returnvalue_scale) (`KismetMathLibrary.BreakTransform` (`SceneComponent.GetRelativeTransform` (`self.Button1`))))
  (set `self.ButtonOut` (`KismetMathLibrary.MakeTransform` _returnvalue_location _returnvalue_rotation _returnvalue_scale))
  (set `self.ButtonIn` (`KismetMathLibrary.MakeTransform` (- _returnvalue_location (0.0 0.0 25.0)) _returnvalue_rotation _returnvalue_scale))
  (`self.EnableInput` (`GameplayStatics.GetPlayerController` 0)))

(event `Key|LeftMouseButton`
  (params (Key :type "Key Structure"))
  (:`Pressed`
    (`/Engine/EditorBlueprintResources/StandardMacros.Gate` true
      (:`Exit`
        (bind (_direction _newtrack_0) (`Timeline|In` :!via `PlayFromStart`)
          (:`Update`
            (`SceneComponent.K2_SetRelativeTransform` (`self.Button1`) (`KismetMathLibrary.TLerp` (`self.ButtonOut`) (`self.ButtonIn`) _newtrack_0) false false))
          (:`Finished`
            (bind (_direction_2 _newtrack_0_2) (`Timeline|Out` :!via `ReverseFromEnd`)
              (:`Update`
                (`SceneComponent.K2_SetRelativeTransform` (`self.Button1`) (`KismetMathLibrary.TLerp` (`self.ButtonOut`) (`self.ButtonIn`) _newtrack_0_2) false false)))))))))

(event `self.Collision1.OnComponentBeginOverlap`
  (params (OverlappedComponent :type "PrimitiveComponent Object Reference") (OtherActor :type "Actor Object Reference") (OtherComp :type "PrimitiveComponent Object Reference") (OtherBodyIndex :type Integer) (bFromSweep :type Boolean) (SweepResult :type "HitResult Structure (by ref)")))

(event `self.Collision1.OnComponentEndOverlap`
  (params (OverlappedComponent :type "PrimitiveComponent Object Reference") (OtherActor :type "Actor Object Reference") (OtherComp :type "PrimitiveComponent Object Reference") (OtherBodyIndex :type Integer)))

(fn `UserConstructionScript`)