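; Shader engine Blueprint that animates eight sphere components in continuous back-and-forth motion.
; BeginPlay starts one custom event per sphere, each looping endlessly between two hardcoded relative locations through chained MoveComponentTo latent moves.
; The first four spheres zigzag in the X-Z plane, while the other four mainly swing diagonally across X and Y.
; All moves share the MoveOverTime duration, and the construction script is empty.
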(event `self.ReceiveBeginPlay`
  (`self.SphereMove`)
  (`self.Sphere1Move`)
  (`self.Sphere2Move`)
  (`self.Sphere3Move`)
  (`self.Sphere4Move`)
  (`self.Sphere5Move`)
  (`self.Sphere6Move`)
  (`self.Sphere7Move`))

(event `SphereMove`
  (bind _sphere (`self.Sphere`))
  (bind _moveovertime (`self.MoveOverTime`))
  (`KismetSystemLibrary.MoveComponentTo` _sphere (-200.0 0.0 54.0) (struct) false false _moveovertime :!label _label)
  (`KismetSystemLibrary.MoveComponentTo` _sphere (-100.0 0.0 -54.0) (struct) false false _moveovertime)
  (goto _label))

(event `Sphere1Move`
  (bind _sphere1 (`self.Sphere1`))
  (bind _moveovertime (`self.MoveOverTime`))
  (`KismetSystemLibrary.MoveComponentTo` _sphere1 (-100.0 0.0 -54.0) (struct) false false _moveovertime :!label _label_2)
  (`KismetSystemLibrary.MoveComponentTo` _sphere1 (0.0 0.0 54.0) (struct) false false _moveovertime)
  (goto _label_2))

(event `Sphere2Move`
  (bind _sphere2 (`self.Sphere2`))
  (bind _moveovertime (`self.MoveOverTime`))
  (`KismetSystemLibrary.MoveComponentTo` _sphere2 (0.0 0.0 54.0) (struct) false false _moveovertime :!label _label_3)
  (`KismetSystemLibrary.MoveComponentTo` _sphere2 (100.0 0.0 -54.0) (struct) false false _moveovertime)
  (goto _label_3))

(event `Sphere3Move`
  (bind _sphere3 (`self.Sphere3`))
  (bind _moveovertime (`self.MoveOverTime`))
  (`KismetSystemLibrary.MoveComponentTo` _sphere3 (100.0 0.0 -54.0) (struct) false false _moveovertime :!label _label_4)
  (`KismetSystemLibrary.MoveComponentTo` _sphere3 (200.0 0.0 54.0) (struct) false false _moveovertime)
  (goto _label_4))

(event `Sphere4Move`
  (bind _sphere4 (`self.Sphere4`))
  (bind _moveovertime (`self.MoveOverTime`))
  (`KismetSystemLibrary.MoveComponentTo` _sphere4 (0.0 50.0 40.0) (struct) false false _moveovertime :!label _label_5)
  (`KismetSystemLibrary.MoveComponentTo` _sphere4 (100.0 -50.0 40.0) (struct) false false _moveovertime)
  (goto _label_5))

(event `Sphere5Move`
  (bind _sphere5 (`self.Sphere5`))
  (bind _moveovertime (`self.MoveOverTime`))
  (`KismetSystemLibrary.MoveComponentTo` _sphere5 (200.0 50.0 40.0) (struct) false false _moveovertime :!label _label_6)
  (`KismetSystemLibrary.MoveComponentTo` _sphere5 (100.0 -50.0 40.0) (struct) false false _moveovertime)
  (goto _label_6))

(event `Sphere6Move`
  (bind _sphere6 (`self.Sphere6`))
  (bind _moveovertime (`self.MoveOverTime`))
  (`KismetSystemLibrary.MoveComponentTo` _sphere6 (-100.0 -50.0 40.0) (struct) false false _moveovertime :!label _label_7)
  (`KismetSystemLibrary.MoveComponentTo` _sphere6 (0.0 50.0 40.0) (struct) false false _moveovertime)
  (goto _label_7))

(event `Sphere7Move`
  (bind _sphere7 (`self.Sphere7`))
  (bind _moveovertime (`self.MoveOverTime`))
  (`KismetSystemLibrary.MoveComponentTo` _sphere7 (100.0 -50.0 -40.0) (struct) false false _moveovertime :!label _label_8)
  (`KismetSystemLibrary.MoveComponentTo` _sphere7 (0.0 50.0 40.0) (struct) false false _moveovertime)
  (goto _label_8))

(fn `UserConstructionScript`)