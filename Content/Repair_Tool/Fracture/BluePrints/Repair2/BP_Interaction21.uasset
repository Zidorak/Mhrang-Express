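; BP_Interaction21 is an interactable repair point that shows a prompt widget while its collision volume is overlapped.
; Interact alternates through a FlipFlop between playing a timeline and resetting its time; the timeline drives Alpha3 in the PC_TimeReversal parameter collection while freezing player movement.
; On finish it restores walking, hides the prompt, sets Disable, calls Repair on BP_TimerZone2 and turns off its collision.
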(event `self.Interact`
  (`/Engine/EditorBlueprintResources/StandardMacros.FlipFlop`
    (:`A`
      (bind (_direction _newtrack_0) (`Timeline|Timeline` :`NewTime` 1.0 :!label _label)
        (:`Update`
          (bind _returnvalue (`GameplayStatics.GetActorOfClass` "/Game/FirstPerson/Blueprints/BP_FirstPersonCharacter.BP_FirstPersonCharacter_C"))
          (`CharacterMovementComponent.SetMovementMode` (`Character.CharacterMovement` _returnvalue) "MOVE_None" 0)
          (`KismetMaterialLibrary.SetScalarParameterValue` "/Game/Repair_Tool/Fracture/BluePrints/PC_TimeReversal.PC_TimeReversal" "Alpha3" _newtrack_0))
        (:`Finished`
          (bind _returnvalue_2 (`GameplayStatics.GetActorOfClass` "/Game/FirstPerson/Blueprints/BP_FirstPersonCharacter.BP_FirstPersonCharacter_C"))
          (`CharacterMovementComponent.SetMovementMode` (`Character.CharacterMovement` _returnvalue_2) "MOVE_Walking" 0)
          (`SceneComponent.SetVisibility` (`self.Widget`) false false)
          (set `self.Disable` true)
          (bind _returnvalue_3 (`GameplayStatics.GetActorOfClass` "/Game/Repair_Tool/Fracture/BluePrints/Repair2/BP_TimerZone2.BP_TimerZone2_C"))
          (`/Game/Repair_Tool/Fracture/BluePrints/BI_Repair.Repair` _returnvalue_3)
          (`PrimitiveComponent.SetCollisionEnabled` (`self.Collision`) "NoCollision")
          (goto _label :!via `Stop`))))
    (:`B`
      (goto _label :!via `SetNewTime`))))

(event `self.Collision.OnComponentBeginOverlap`
  (params (OverlappedComponent :type "PrimitiveComponent Object Reference") (OtherActor :type "Actor Object Reference") (OtherComp :type "PrimitiveComponent Object Reference") (OtherBodyIndex :type Integer) (bFromSweep :type Boolean) (SweepResult :type "HitResult Structure (by ref)"))
  (`SceneComponent.SetVisibility` (`self.Widget`) true false))

(event `self.Collision.OnComponentEndOverlap`
  (params (OverlappedComponent :type "PrimitiveComponent Object Reference") (OtherActor :type "Actor Object Reference") (OtherComp :type "PrimitiveComponent Object Reference") (OtherBodyIndex :type Integer))
  (`SceneComponent.SetVisibility` (`self.Widget`) false false))

(fn `UserConstructionScript`)