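; BP_TimerZone2 is a repair-zone trigger that starts a timed challenge, showing WB_Lose if the player character's Seconds reach zero.
; Overlapping the box shows the countdown widget, starts breathing audio and switches BP_DoorEngine2's collision location off.
; Tick drives CountDown, using a Delay to pace each decrement.
; Repair checks both interaction actors' disable flags, then stops and resets the timer, disables the box, hides the widget and reverses the door and audio changes.
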(event `self.Repair`
  (bind _returnvalue (`GameplayStatics.GetActorOfClass` "/Game/Repair_Tool/Fracture/BluePrints/Repair2/BP_Interaction21.BP_Interaction21_C"))
  (bind _returnvalue_2 (`GameplayStatics.GetActorOfClass` "/Game/Repair_Tool/Fracture/BluePrints/Repair2/BP_Interaction22.BP_Interaction22_C"))
  (if (and (`/Game/Repair_Tool/Fracture/BluePrints/Repair2/BP_Interaction21.Disable` _returnvalue) (`/Game/Repair_Tool/Fracture/BluePrints/Repair2/BP_Interaction22.Disable2` _returnvalue_2))
    (set `self.Repaired` true)
    (if (`self.Repaired`)
      (`self.Timer`)
      (`PrimitiveComponent.SetCollisionEnabled` (`self.Box`) "NoCollision")
      (`KismetSystemLibrary.Delay` 1.0)
      (bind _foundwidgets (`WidgetBlueprintLibrary.GetAllWidgetsOfClass` "/Game/Repair_Tool/Fracture/BluePrints/Widgets/WB_CountDownTimer.WB_CountDownTimer_C"))
      (`Widget.SetVisibility` _foundwidgets "Hidden")
      (bind _returnvalue_3 (`GameplayStatics.GetActorOfClass` "/Game/Repair_Tool/DoorCollision/BP_DoorEngine2.BP_DoorEngine2_C"))
      (`/Game/Repair_Tool/DoorCollision/BP_DoorEngine2.CollisionLocationDoorON` _returnvalue_3)
      (bind _returnvalue_4 (`GameplayStatics.GetActorOfClass` "/Game/Repair_Tool/Music/Breathing/BP_breathing2.BP_breathing2_C"))
      (`/Game/Repair_Tool/Music/Breathing/BP_breathing2.EndSound` _returnvalue_4))))

(event `CountDown`
  (`KismetSystemLibrary.Delay` 1.0)
  (if (not (`self.TimerOn`))
    (bind _returnvalue (`GameplayStatics.GetActorOfClass` "/Game/FirstPerson/Blueprints/BP_FirstPersonCharacter.BP_FirstPersonCharacter_C"))
    (if (== 0 (`/Game/FirstPerson/Blueprints/BP_FirstPersonCharacter.Seconds` _returnvalue))
      (bind _returnvalue_2 (`|CreateWidget` "/Game/Repair_Tool/UI/WB_Lose.WB_Lose_C"))
      (`UserWidget.AddToViewport` _returnvalue_2 0)
      (else
        (set `/Game/FirstPerson/Blueprints/BP_FirstPersonCharacter.Seconds` (- (`/Game/FirstPerson/Blueprints/BP_FirstPersonCharacter.Seconds` _returnvalue) 1) _returnvalue)))))

(event `self.ReceiveTick`
  (params (DeltaSeconds :type "Float (single-precision)"))
  (if (`self.Count`)
    (`self.CountDown`)))

(event `self.Box.OnComponentBeginOverlap`
  (params (OverlappedComponent :type "PrimitiveComponent Object Reference") (OtherActor :type "Actor Object Reference") (OtherComp :type "PrimitiveComponent Object Reference") (OtherBodyIndex :type Integer) (bFromSweep :type Boolean) (SweepResult :type "HitResult Structure (by ref)"))
  (set `self.Count` true)
  (`self.CountDown`)
  (bind _returnvalue (`|CreateWidget` "/Game/Repair_Tool/Fracture/BluePrints/Widgets/WB_CountDownTimer.WB_CountDownTimer_C"))
  (`UserWidget.AddToViewport` _returnvalue 0)
  (bind _foundwidgets (`WidgetBlueprintLibrary.GetAllWidgetsOfClass` "/Game/Repair_Tool/Fracture/BluePrints/Widgets/WB_CountDownTimer.WB_CountDownTimer_C"))
  (`Widget.SetVisibility` _foundwidgets "Visible")
  (bind _returnvalue_2 (`GameplayStatics.GetActorOfClass` "/Game/Repair_Tool/DoorCollision/BP_DoorEngine2.BP_DoorEngine2_C"))
  (`/Game/Repair_Tool/DoorCollision/BP_DoorEngine2.CollisionLocationOff` _returnvalue_2)
  (bind _returnvalue_3 (`GameplayStatics.GetActorOfClass` "/Game/Repair_Tool/Music/Breathing/BP_breathing2.BP_breathing2_C"))
  (`/Game/Repair_Tool/Music/Breathing/BP_breathing2.SoundOn` _returnvalue_3))

(event `Timer`
  (set `self.TimerOn` true)
  (bind _returnvalue (`GameplayStatics.GetActorOfClass` "/Game/FirstPerson/Blueprints/BP_FirstPersonCharacter.BP_FirstPersonCharacter_C"))
  (set `/Game/FirstPerson/Blueprints/BP_FirstPersonCharacter.Seconds` 30 _returnvalue))

(fn `UserConstructionScript`)