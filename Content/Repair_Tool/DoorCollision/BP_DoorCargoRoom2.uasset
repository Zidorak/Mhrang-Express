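; Sliding double door for Cargo Room 2 that moves its two leaves in opposite directions through a Timeline.
; Begin and end overlaps on both trigger volumes share one FlipFlop, alternately playing and reversing the Timeline rather than tracking occupancy.
; Collision1 and StripFinal start off.
; A Destroy event disables Collision and shows StripFinal, while a Create event enables Collision1 and hides it, without re-enabling Collision.
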(event `self.Collision.OnComponentBeginOverlap`
  (params (OverlappedComponent :type "PrimitiveComponent Object Reference") (OtherActor :type "Actor Object Reference") (OtherComp :type "PrimitiveComponent Object Reference") (OtherBodyIndex :type Integer) (bFromSweep :type Boolean) (SweepResult :type "HitResult Structure (by ref)"))
  (`/Engine/EditorBlueprintResources/StandardMacros.FlipFlop` :!label _label
    (:`A`
      (bind (_direction _close) (`Timeline|Timeline` :`NewTime` 5.0 :!label _label_2)
        (:`Update`
          (`SceneComponent.K2_SetRelativeLocation` (`self.left_door`) (`KismetMathLibrary.MakeVector` (`KismetMathLibrary.Lerp` -700.0 -500.0 _close)) false false)
          (`SceneComponent.K2_SetRelativeLocation` (`self.right_door`) (`KismetMathLibrary.MakeVector` (`KismetMathLibrary.Lerp` -700.0 -900.0 _close)) false false))))
    (:`B`
      (goto _label_2 :!via `Reverse`))))

(event `self.Collision.OnComponentEndOverlap`
  (params (OverlappedComponent :type "PrimitiveComponent Object Reference") (OtherActor :type "Actor Object Reference") (OtherComp :type "PrimitiveComponent Object Reference") (OtherBodyIndex :type Integer))
  (goto _label))

(event `self.Collision1.OnComponentBeginOverlap`
  (params (OverlappedComponent :type "PrimitiveComponent Object Reference") (OtherActor :type "Actor Object Reference") (OtherComp :type "PrimitiveComponent Object Reference") (OtherBodyIndex :type Integer) (bFromSweep :type Boolean) (SweepResult :type "HitResult Structure (by ref)"))
  (goto _label))

(event `self.ReceiveBeginPlay`
  (`PrimitiveComponent.SetCollisionEnabled` (`self.Collision1`) "NoCollision")
  (`SceneComponent.SetVisibility` (`self.Strip_final`) false false))

(event `self.Collision1.OnComponentEndOverlap`
  (params (OverlappedComponent :type "PrimitiveComponent Object Reference") (OtherActor :type "Actor Object Reference") (OtherComp :type "PrimitiveComponent Object Reference") (OtherBodyIndex :type Integer))
  (goto _label))

(event `Destroy`
  (`PrimitiveComponent.SetCollisionEnabled` (`self.Collision`) "NoCollision")
  (`SceneComponent.SetVisibility` (`self.Strip_final`) true false))

(event `Create`
  (`PrimitiveComponent.SetCollisionEnabled` (`self.Collision1`) "QueryAndPhysics")
  (`SceneComponent.SetVisibility` (`self.Strip_final`) false false))

(fn `UserConstructionScript`)