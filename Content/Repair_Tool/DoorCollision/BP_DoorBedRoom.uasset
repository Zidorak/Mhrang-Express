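; BP_DoorBedRoom is a bedroom double sliding door that stays inactive until CollisionLocationDoorON is called.
; Begin and end overlaps on its Collision volume share one FlipFlop, alternately playing and reversing a Timeline that slides LeftDoor and RightDoor in opposite directions along X.
; On BeginPlay a Timeline lowers the Collision far below the door; CollisionLocationDoorON raises it back and hides StripFinal.
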(event `self.Collision.OnComponentBeginOverlap`
  (params (OverlappedComponent :type "PrimitiveComponent Object Reference") (OtherActor :type "Actor Object Reference") (OtherComp :type "PrimitiveComponent Object Reference") (OtherBodyIndex :type Integer) (bFromSweep :type Boolean) (SweepResult :type "HitResult Structure (by ref)"))
  (`/Engine/EditorBlueprintResources/StandardMacros.FlipFlop` :!label _label
    (:`A`
      (bind (_direction _close) (`Timeline|Timeline` :`NewTime` 5.0 :!label _label_2)
        (:`Update`
          (`SceneComponent.K2_SetRelativeLocation` (`self.left_door`) (`KismetMathLibrary.MakeVector` (`KismetMathLibrary.Lerp` -700.0 -500.0 _close)) false false)
          (`SceneComponent.K2_SetRelativeLocation` (`self.right_door`) (`KismetMathLibrary.MakeVector` (`KismetMathLibrary.Lerp` -700.0 -900.0 _close)) false false))))
    (:`B`
      (goto _label_2 :!via `Reverse`))))

(event `self.Collision.OnComponentEndOverlap`
  (params (OverlappedComponent :type "PrimitiveComponent Object Reference") (OtherActor :type "Actor Object Reference") (OtherComp :type "PrimitiveComponent Object Reference") (OtherBodyIndex :type Integer))
  (goto _label))

(event `self.ReceiveBeginPlay`
  (bind (_direction _newtrack_0) (`Timeline|Timeline_0`)
    (:`Update`
      (`SceneComponent.K2_SetRelativeLocation` (`self.Collision`) (`KismetMathLibrary.MakeVector` 0.0 30.0 (`KismetMathLibrary.Lerp` 0.0 -1000.0 _newtrack_0)) true true))))

(event `CollisionLocationDoorON`
  (bind (_direction _newtrack_0) (`Timeline|Timeline_1`)
    (:`Update`
      (`SceneComponent.K2_SetRelativeLocation` (`self.Collision`) (`KismetMathLibrary.MakeVector` 0.0 30.0 (`KismetMathLibrary.Lerp` -1000.0 0.0 _newtrack_0)) true true)
      (`SceneComponent.SetVisibility` (`self.Strip_final`) false false))))

(fn `UserConstructionScript`)