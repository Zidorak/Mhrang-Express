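; BP_DoorRegularSmall is a small sliding double door that moves when something overlaps its Collision component.
; Begin and end overlap share one FlipFlop, alternately playing and reversing a Timeline that lerps both leaves apart along X, regardless of which event fired.
; Custom events ColOff and ColOn respectively disable the trigger and enable a second component, Collision1, which starts disabled on BeginPlay.
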(event `self.Collision.OnComponentBeginOverlap`
  (params (OverlappedComponent :type "PrimitiveComponent Object Reference") (OtherActor :type "Actor Object Reference") (OtherComp :type "PrimitiveComponent Object Reference") (OtherBodyIndex :type Integer) (bFromSweep :type Boolean) (SweepResult :type "HitResult Structure (by ref)"))
  (`/Engine/EditorBlueprintResources/StandardMacros.FlipFlop` :!label _label
    (:`A`
      (bind (_direction _close) (`Timeline|Timeline` :`NewTime` 5.0 :!label _label_2)
        (:`Update`
          (`SceneComponent.K2_SetRelativeLocation` (`self.left_door`) (`KismetMathLibrary.MakeVector` (`KismetMathLibrary.Lerp` 50.0 150.0 _close)) false false)
          (`SceneComponent.K2_SetRelativeLocation` (`self.right_door`) (`KismetMathLibrary.MakeVector` (`KismetMathLibrary.Lerp` -50.0 -150.0 _close)) false false))))
    (:`B`
      (goto _label_2 :!via `Reverse`))))

(event `self.Collision.OnComponentEndOverlap`
  (params (OverlappedComponent :type "PrimitiveComponent Object Reference") (OtherActor :type "Actor Object Reference") (OtherComp :type "PrimitiveComponent Object Reference") (OtherBodyIndex :type Integer))
  (goto _label))

(event `self.ReceiveBeginPlay`
  (`PrimitiveComponent.SetCollisionEnabled` (`self.Collision1`) "NoCollision"))

(event `ColOff`
  (`PrimitiveComponent.SetCollisionEnabled` (`self.Collision`) "NoCollision"))

(event `ColOn`
  (`PrimitiveComponent.SetCollisionEnabled` (`self.Collision1`) "QueryAndPhysics"))

(fn `UserConstructionScript`)