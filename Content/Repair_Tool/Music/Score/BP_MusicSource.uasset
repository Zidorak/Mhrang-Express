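; BP_MusicSource drives a dynamic music score through timed stages of start, middle, end and finished.
; Its Start event runs a linear chain of fixed Delays lasting about six minutes, firing trigger parameters on the Audio component at each stage.
; A siren trigger switches on with the end stage and off when the score finishes.
; BeginPlay is empty, so the sequence waits for Start to be called.
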(event `self.ReceiveBeginPlay`)

(event `Start`
  (bind _audio (`self.Audio`))
  ;[1 1 1] Play music dynamically
  (`KismetSystemLibrary.Delay` 1.0)
  (`AudioParameterControllerInterface.SetTriggerParameter` _audio "OnStart")
  (`KismetSystemLibrary.Delay` 180.0)
  (`AudioParameterControllerInterface.SetTriggerParameter` _audio "OnMiddle")
  (`KismetSystemLibrary.Delay` 90.0)
  (`AudioParameterControllerInterface.SetTriggerParameter` _audio "SirenOn")
  (`AudioParameterControllerInterface.SetTriggerParameter` _audio "OnEnd")
  (`KismetSystemLibrary.Delay` 90.0)
  (`AudioParameterControllerInterface.SetTriggerParameter` _audio "OnFinished")
  (`AudioParameterControllerInterface.SetTriggerParameter` _audio "SirenOff"))

(fn `UserConstructionScript`)