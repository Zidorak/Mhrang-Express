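; BP_Buttons is a single keypad button that highlights under the cursor and reports clicks to its keypad.
; Cursor-over events swap the Button component's material between M_On and M_Base, and ResetButtons restores the base material.
; A click calls ButtonEntered on KeypadActorRef, passing the button's NoText value with its confirm and backspace flags.
; The construction script displays NoText on the button's Button0 label.
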(event `self.Button.OnBeginCursorOver`
  (params (TouchedComponent :type "PrimitiveComponent Object Reference"))
  (`PrimitiveComponent.SetMaterial` (`self.Button`) 0 "/Game/Repair_Tool/Keypad/Materials/M_On.M_On"))

(event `self.Button.OnEndCursorOver`
  (params (TouchedComponent :type "PrimitiveComponent Object Reference"))
  (`PrimitiveComponent.SetMaterial` (`self.Button`) 0 "/Game/Repair_Tool/Keypad/Materials/M_Base.M_Base" :!label _label))

(event `Reset Buttons`
  (goto _label))

(event `self.Button.OnClicked`
  (params (TouchedComponent :type "PrimitiveComponent Object Reference") (ButtonPressed :type "Key Structure"))
  (`/Game/Repair_Tool/Keypad/BluePrintsKeypad/BP_Keypad.Button entered` (`self.KeypadActorRef`) (`self.NoText`) (`self.ConfirmedButton`) (`self.BackspaceButton`)))

(fn `UserConstructionScript`
  (`TextRenderComponent.K2_SetText` (`self.Button0`) (`self.NoText`)))