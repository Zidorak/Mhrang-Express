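; BP_Keypad is an interactable code-entry keypad that opens the BP_ButtonsPanel when the correct code is entered.
; Its Box overlap registers it with the first-person character, and OnInteract switches to the keypad camera with mouse clicking and links twelve child-actor buttons to itself.
; Buttons feed digit, backspace and confirm into a text render, which OnConfirmed compares to CorrectCode.
; After coloured feedback and a delay, it restores the player view, HUD and gun.
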(event `self.Box.OnComponentBeginOverlap`
  (params (OverlappedComponent :type "PrimitiveComponent Object Reference") (OtherActor :type "Actor Object Reference") (OtherComp :type "PrimitiveComponent Object Reference") (OtherBodyIndex :type Integer) (bFromSweep :type Boolean) (SweepResult :type "HitResult Structure (by ref)"))
  (if (== OtherActor (`GameplayStatics.GetPlayerPawn` 0))
    (bind _asbp_first_person_character (cast `/Game/FirstPerson/Blueprints/BP_FirstPersonCharacter` OtherActor))
    (set `/Game/FirstPerson/Blueprints/BP_FirstPersonCharacter.KeypadInteractActor` self _asbp_first_person_character)
    (set `self.Player Ref` _asbp_first_person_character)))

(event `self.Box.OnComponentEndOverlap`
  (params (OverlappedComponent :type "PrimitiveComponent Object Reference") (OtherActor :type "Actor Object Reference") (OtherComp :type "PrimitiveComponent Object Reference") (OtherBodyIndex :type Integer))
  (if (== OtherActor (`GameplayStatics.GetPlayerPawn` 0))
    (bind _asbp_first_person_character (cast `/Game/FirstPerson/Blueprints/BP_FirstPersonCharacter` OtherActor))
    (set `/Game/FirstPerson/Blueprints/BP_FirstPersonCharacter.KeypadInteractActor` null _asbp_first_person_character)
    (set `self.Player Ref` null)))

(event `OnInteract`
  (bind _returnvalue (`GameplayStatics.GetPlayerController` 0))
  (bind _entercode (`self.EnterCode`))
  (bind _returnvalue_2 (`GameplayStatics.GetActorOfClass` "/Game/FirstPerson/Blueprints/BP_FirstPersonCharacter.BP_FirstPersonCharacter_C"))
  (`/Game/FirstPerson/Blueprints/BP_FirstPersonCharacter.GunVisibility` _returnvalue_2)
  (`PlayerController.SetViewTargetWithBlend` (`GameplayStatics.GetPlayerController` 0) (`ActorComponent.GetOwner` (`self.CameraKeypad`)) 0.0 "VTBlend_Linear" 0.0 false)
  (bind _output_get (set `PlayerController.bShowMouseCursor` true _returnvalue :!label _label))
  (bind _output_get_2 (set `PlayerController.bEnableClickEvents` _output_get _returnvalue))
  (set `PlayerController.bEnableMouseOverEvents` _output_get_2 _returnvalue)
  (`TextRenderComponent.K2_SetText` _entercode "")
  (`TextRenderComponent.SetTextRenderColor` _entercode (make `Color` 1 1 1 255))
  (bind _output_get_3 (set `self.ButtonsArray` (`|MakeArray` (`self.Button1`) (`self.Button2`) (`self.Button3`) (`self.Button4`) (`self.Button5`) (`self.Button6`) (`self.Button7`) (`self.Button8`) (`self.Button9`) (`self.ButtonBack`) (`self.Button0`) (`self.ButtonConfirm`))))
  (for _array_element _output_get_3
    (bind _asbp_buttons (cast `/Game/Repair_Tool/Keypad/BluePrintsKeypad/BP_Buttons` (`ChildActorComponent.ChildActor` _array_element)))
    (set `/Game/Repair_Tool/Keypad/BluePrintsKeypad/BP_Buttons.KeypadActorRef` self _asbp_buttons)))

(event `Initiate`
  (goto _label))

(event `Button entered`
  (params (Value :type Text) (`Confirmed?` :type Boolean) (Backspace :type Boolean))
  (bind _entercode (`self.EnterCode`))
  (if `Confirmed?`
    (`self.On Confirmed`)
    (elif Backspace
      (`self.Backspace`)
      (elif (`self.Can Enter`)
        (`TextRenderComponent.K2_SetText` _entercode (`KismetTextLibrary.Conv_StringToText` (`KismetStringLibrary.Replace` (`KismetTextLibrary.Conv_TextToString` (`TextRenderComponent.Text` (`self.EnterCode`))) (`KismetStringLibrary.GetSubstring` "...." 0 (`KismetStringLibrary.Len` (`self.CorrectCode`))))))
        (`TextRenderComponent.K2_SetText` _entercode (`KismetTextLibrary.Conv_StringToText` (`KismetStringLibrary.Concat_StrStr` (`KismetTextLibrary.Conv_TextToString` (`TextRenderComponent.Text` (`self.EnterCode`))) (`KismetTextLibrary.Conv_TextToString` Value))))
        (`TextRenderComponent.SetTextRenderColor` (`self.EnterCode`) (make `Color` 255 255 255 255))))))

(event `Backspace`
  (bind _entercode (`self.EnterCode`))
  (bind _returnvalue (`KismetTextLibrary.Conv_TextToString` (`TextRenderComponent.Text` _entercode)))
  (`TextRenderComponent.K2_SetText` _entercode (`KismetTextLibrary.Conv_StringToText` (`KismetStringLibrary.GetSubstring` _returnvalue 0 (- (`KismetStringLibrary.Len` _returnvalue) 1)))))

(event `On Confirmed`
  (bind _returnvalue (`GameplayStatics.GetPlayerController` 0))
  (bind _returnvalue_2 (`GameplayStatics.GetPlayerController` 0))
  (bind _entercode (`self.EnterCode`))
  (bind _entercode_2 (`self.EnterCode`))
  (if (`KismetStringLibrary.EqualEqual_StrStr` (`KismetTextLibrary.Conv_TextToString` (`TextRenderComponent.Text` (`self.EnterCode`))) (`self.CorrectCode`))
    (`|ExecutionSequence`
      (:`then_0`
        (`TextRenderComponent.K2_SetText` _entercode_2 "Correct code")
        (`TextRenderComponent.SetTextRenderColor` _entercode_2 (make `Color` 0 255 0 255))
        (`KismetSystemLibrary.RetriggerableDelay` 2.0)
        (bind _output_get (set `PlayerController.bShowMouseCursor` false _returnvalue_2))
        (bind _output_get_2 (set `PlayerController.bEnableMouseOverEvents` _output_get _returnvalue_2))
        (set `PlayerController.bEnableClickEvents` _output_get_2 _returnvalue_2)
        (for _array_element (`self.ButtonsArray`)
          (bind _asbp_buttons (cast `/Game/Repair_Tool/Keypad/BluePrintsKeypad/BP_Buttons` (`ChildActorComponent.ChildActor` _array_element)))
          (`/Game/Repair_Tool/Keypad/BluePrintsKeypad/BP_Buttons.Reset Buttons` _asbp_buttons))
        (`PlayerController.SetViewTargetWithBlend` (`GameplayStatics.GetPlayerController` 0) (`ActorComponent.GetOwner` (`/Game/FirstPerson/Blueprints/BP_FirstPersonCharacter.FirstPersonCamera` (cast `/Game/FirstPerson/Blueprints/BP_FirstPersonCharacter` (`GameplayStatics.GetPlayerPawn` 0) :!pure true))) 0.4 "VTBlend_Linear" 0.0 false)
        (`TextRenderComponent.K2_SetText` (`self.EnterCode`) "")
        (`WidgetBlueprintLibrary.SetInputMode_GameOnly` (`GameplayStatics.GetPlayerController` 0))
        (bind _returnvalue_3 (`GameplayStatics.GetActorOfClass` "/Game/PuzzleGameProject/PuzzlesBPs/ControlRoom/BP_ButtonsPanel.BP_ButtonsPanel_C"))
        (`/Game/PuzzleGameProject/PuzzlesBPs/ControlRoom/BP_ButtonsPanel.OpenUp` _returnvalue_3)
        (`ActorComponent.K2_DestroyComponent` (`self.Box`))
        (bind _foundwidgets (`WidgetBlueprintLibrary.GetAllWidgetsOfClass` "/Game/Repair_Tool/HUD_Paralax/WB_HUD.WB_HUD_C"))
        (`Widget.SetVisibility` _foundwidgets "Visible")
        (bind _returnvalue_4 (`GameplayStatics.GetActorOfClass` "/Game/FirstPerson/Blueprints/BP_FirstPersonCharacter.BP_FirstPersonCharacter_C"))
        (`/Game/FirstPerson/Blueprints/BP_FirstPersonCharacter.GunVisibilityOn` _returnvalue_4))
      (:`then_1`
        (set `self.Can Enter` false)))
    (else
      (`|ExecutionSequence`
        (:`then_0`
          (`TextRenderComponent.K2_SetText` _entercode "Wrong code")
          (`TextRenderComponent.SetTextRenderColor` _entercode (make `Color` 0 0 255 255))
          (`KismetSystemLibrary.RetriggerableDelay` 2.0)
          (bind _output_get_3 (set `PlayerController.bEnableMouseOverEvents` false _returnvalue))
          (set `PlayerController.bEnableClickEvents` _output_get_3 _returnvalue)
          (for _array_element_2 (`self.ButtonsArray`)
            (bind _asbp_buttons_2 (cast `/Game/Repair_Tool/Keypad/BluePrintsKeypad/BP_Buttons` (`ChildActorComponent.ChildActor` _array_element_2)))
            (`/Game/Repair_Tool/Keypad/BluePrintsKeypad/BP_Buttons.Reset Buttons` _asbp_buttons_2)
            (set `self.Can Enter` true))
          (`PlayerController.SetViewTargetWithBlend` (`GameplayStatics.GetPlayerController` 0) (`ActorComponent.GetOwner` (`/Game/FirstPerson/Blueprints/BP_FirstPersonCharacter.FirstPersonCamera` (cast `/Game/FirstPerson/Blueprints/BP_FirstPersonCharacter` (`GameplayStatics.GetPlayerPawn` 0) :!pure true))) 0.4 "VTBlend_Linear" 0.0 false)
          (`self.Initiate`)
          (set `PlayerController.bShowMouseCursor` false _returnvalue)
          (bind _foundwidgets_2 (`WidgetBlueprintLibrary.GetAllWidgetsOfClass` "/Game/Repair_Tool/HUD_Paralax/WB_HUD.WB_HUD_C"))
          (`Widget.SetVisibility` _foundwidgets_2 "Visible")
          (bind _returnvalue_5 (`GameplayStatics.GetActorOfClass` "/Game/FirstPerson/Blueprints/BP_FirstPersonCharacter.BP_FirstPersonCharacter_C"))
          (`/Game/FirstPerson/Blueprints/BP_FirstPersonCharacter.GunVisibilityOn` _returnvalue_5))
        (:`then_1`
          (set `self.Can Enter` false))))))

(fn `UserConstructionScript`)