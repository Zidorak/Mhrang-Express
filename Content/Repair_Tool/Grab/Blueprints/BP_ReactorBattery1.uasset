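; BP_ReactorBattery1 is a reactor battery actor in the repair tool's grab content that switches to a second state when its Overlap event fires.
; BeginPlay hides Cylinder and disables its collision.
; Overlap sets a True flag, hides Cylinder1, and shows Cylinder with query and physics collision.
; It then snaps the actor to its Rotation and Location variables, apparently seating the battery in place.
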(event `Overlap`
  (bind _cylinder (`self.Cylinder`))
  (bind _cylinder1 (`self.Cylinder1`))
  (set `self.True` true)
  (`SceneComponent.SetVisibility` _cylinder1 false false)
  (`PrimitiveComponent.SetCollisionEnabled` _cylinder1 "NoCollision")
  (`SceneComponent.SetVisibility` _cylinder true false)
  (`PrimitiveComponent.SetCollisionEnabled` _cylinder "QueryAndPhysics")
  (`self.K2_SetActorRotation` (`self.Rotation`))
  (`self.K2_SetActorLocation` (`self.Location`)))

(event `self.ReceiveBeginPlay`
  (bind _cylinder (`self.Cylinder`))
  (`SceneComponent.SetVisibility` _cylinder false false)
  (`PrimitiveComponent.SetCollisionEnabled` _cylinder "NoCollision"))

(fn `UserConstructionScript`)