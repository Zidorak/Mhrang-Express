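; BP_PressurePlate2 is a trigger that powers up an engine when an actor tagged GreenReactor overlaps it.
; The overlap notifies BP_ReactorBattery2, then after a short delay plays a startup sound and powers on BP_SoundObject2.
; A FlipFlop's first pass slides Cube1 by timeline, then flags PoweredUp, messages BP_Engine1, disables Box collision and swaps BP_ShaderEngine2's material.
; Target actors are found by class lookup.
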(event `self.ReceiveActorBeginOverlap`
  (params (OtherActor :type "Actor Object Reference"))
  (if (`self.ActorHasTag` OtherActor "GreenReactor")
    (bind _returnvalue (`GameplayStatics.GetActorOfClass` "/Game/Repair_Tool/Grab/Blueprints/BP_ReactorBattery2.BP_ReactorBattery2_C"))
    (`/Game/Repair_Tool/Grab/Blueprints/BP_ReactorBattery2.Overlap` _returnvalue)
    (`KismetSystemLibrary.Delay` 0.5)
    (`GameplayStatics.PlaySound2D` "/Game/Repair_Tool/Music/EngineStarting.EngineStarting" 1.0 1.0 0.0 null null)
    (bind _returnvalue_2 (`GameplayStatics.GetActorOfClass` "/Game/Repair_Tool/Grab/Blueprints/BP_SoundObject2.BP_SoundObject2_C"))
    (`/Game/Repair_Tool/Grab/Blueprints/BP_SoundObject2.PowerOn` _returnvalue_2)
    (`/Engine/EditorBlueprintResources/StandardMacros.FlipFlop`
      (:`A`
        (bind (_direction _close) (`Timeline|Close` :`NewTime` 5.0 :!label _label)
          (:`Update`
            (`SceneComponent.K2_SetRelativeLocation` (`self.Cube1`) (`KismetMathLibrary.MakeVector` (`KismetMathLibrary.Lerp` -140.0 -5.0 _close) -1.0 90.0) false false))
          (:`Finished`
            (set `self.Powered up` true)
            (bind _returnvalue_3 (`GameplayStatics.GetActorOfClass` "/Game/Repair_Tool/Grab/Blueprints/BP_Engine1.BP_Engine1_C"))
            (message `/Game/Repair_Tool/Grab/Blueprints/BI_Engine.EnginePowerUp` _returnvalue_3)
            (`PrimitiveComponent.SetCollisionEnabled` (`self.Box`) "NoCollision")
            (bind _returnvalue_4 (`GameplayStatics.GetActorOfClass` "/Game/PuzzleGameProject/Shader/Blueprints/BP_ShaderEngine2.BP_ShaderEngine2_C"))
            (`PrimitiveComponent.SetMaterial` (`/Game/PuzzleGameProject/Shader/Blueprints/BP_ShaderEngine2.Cylinder` _returnvalue_4) 0 "/Game/PuzzleGameProject/Shader/MM_EngineShader.MM_EngineShader"))))
      (:`B`
        (goto _label :!via `SetNewTime`)))))

(fn `UserConstructionScript`)