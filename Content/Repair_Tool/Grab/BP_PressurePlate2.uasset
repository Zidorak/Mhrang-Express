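; BP_PressurePlate2 is a one-shot pressure plate trigger that powers up the engine when activated.
; An actor overlap plays the Close timeline, sliding two cubes inward toward each other.
; When it finishes, it sets PoweredUp, sends EnginePowerUpMessage to BP_Engine1 found by class, and disables the box's collision.
; A FlipFlop makes alternate overlaps reset the timeline's time instead of playing it.
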(event `self.ReceiveActorBeginOverlap`
  (params (OtherActor :type "Actor Object Reference"))
  (`/Engine/EditorBlueprintResources/StandardMacros.FlipFlop`
    (:`A`
      (bind (_direction _close) (`Timeline|Close` :`NewTime` 2.0 :!label _label)
        (:`Update`
          (`SceneComponent.K2_SetRelativeLocation` (`self.Cube1`) (`KismetMathLibrary.MakeVector` (`KismetMathLibrary.Lerp` -110.0 -50.0 _close) 50.0 60.0) false false)
          (`SceneComponent.K2_SetRelativeLocation` (`self.Cube`) (`KismetMathLibrary.MakeVector` (`KismetMathLibrary.Lerp` 110.0 50.0 _close) 50.0 60.0) false false))
        (:`Finished`
          (set `self.Powered up` true)
          (bind _returnvalue (`GameplayStatics.GetActorOfClass` "/Game/Repair_Tool/Grab/BP_Engine1.BP_Engine1_C"))
          (message `/Game/Repair_Tool/Grab/BI_Engine.EnginePowerUp` _returnvalue)
          (`PrimitiveComponent.SetCollisionEnabled` (`self.Box`) "NoCollision")
          (goto _label :!via `Stop`))))
    (:`B`
      (goto _label :!via `SetNewTime`))))

(fn `UserConstructionScript`)